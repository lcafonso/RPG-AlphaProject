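; BPC_Quest is a quest component that tracks the active quest and drives its on-screen HUD.
; It creates WB_QuestHUD on BeginPlay, with events that push the quest name and objectives into the widget.
; EliminateEnemy removes the given enemy from each incomplete objective's target list, marking an objective completed by reference when its list empties and notifying the HUD.
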(event Custom|Set%20Active%20Quest%20Text
  (Rendering|Components|TextRender|SetText (Variables|/Game/Quest_System/WB_QuestHUD.WB_QuestHUD_C|GetActiveQuestText (Variables|Default|GetQuest%20HUD%20Widget)) (Utilities|Text|ToText(String) (.Name (Utilities|Struct|BreakS_Quest (Variables|Default|GetactiveQuest))))))

(event Custom|Set%20Objectives
  (Default|FillObjectives (Variables|Default|GetQuest%20HUD%20Widget) (.objectives (Variables|Default|GetactiveQuest))))

(event Custom|Eliminate%20Enemy
  (params (Enemy%20Elimenated :type Actor%20Object%20Reference))
  (for _array_element (.objectives (Variables|Default|GetactiveQuest))
    (if (not (.Completed (Utilities|Struct|BreakS_QuestObjective _array_element)))
      (if (> (Utilities|Array|Length (.ActorstoEliminate (Utilities|Struct|BreakS_QuestObjective _array_element))) 0)
        (Utilities|Array|RemoveItem (.ActorstoEliminate (Utilities|Struct|BreakS_QuestObjective _array_element)) Enemy%20Elimenated)
        (if (== (Utilities|Array|Length (.ActorstoEliminate (Utilities|Struct|BreakS_QuestObjective _array_element))) 0)
          (|SetBy-RefVar _array_element (Utilities|Struct|MakeS_QuestObjective (.NameAim (Utilities|Struct|BreakS_QuestObjective _array_element)) true 0 0))
          (Default|ObjetiveComplete (Variables|Default|GetQuest%20HUD%20Widget) _array_element)
          (Development|PrintString "COMPLETED"))))))

(event EventBeginPlay
  (bind _returnvalue (UserInterface|CreateWidget "/Game/Quest_System/WB_QuestHUD.WB_QuestHUD_C"))
  (bind _output_get (Variables|Default|SetQuest%20HUD%20Widget _returnvalue))
  (UserInterface|Viewport|AddtoViewport _output_get 0))