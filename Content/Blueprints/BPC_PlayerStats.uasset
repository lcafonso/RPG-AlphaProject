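; Player stats component for the third-person character that tracks health, stamina, XP and level.
; Decrease functions return true once health or stamina is depleted, and increases to current values clamp to their max.
; Reaching max XP levels up, resetting XP and raising the next threshold by a fixed amount.
; Each change calls UpdateStatsInfo, which pushes bars and text directly into the owning character's HUD widget.
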(event EventBeginPlay
  (Utilities|FlowControl|DelayUntilNextTick)
  (bind _asbp_third_person_character (Utilities|Casting|CastToBP_ThirdPersonCharacter (Components|GetOwner)))
  (Variables|Default|SetPlayer%20Character%20BP _asbp_third_person_character)
  (CallFunction|UpdateStatsInfo))

(fn DecreaseHealth
  (params (Demage :type Float%20%28double-precision%29))
  (if (not (<= (Variables|Health|GetCurrent%20Health) 0.0))
    (Variables|Health|SetCurrent%20Health (- (Variables|Health|GetCurrent%20Health) Demage))
    (CallFunction|UpdateStatsInfo)
    (if (<= (Variables|Health|GetCurrent%20Health) 0.0)
      _
      (else
        (return false))))
  (return true))

(fn IncreaseMaxHealth
  (params (Healt%20Incremention :type Float%20%28double-precision%29))
  (Variables|Health|SetMax%20Health (+ (Variables|Health|GetMax%20Health) Healt%20Incremention))
  (CallFunction|UpdateStatsInfo))

(fn DecreaseStamina
  (params (Stamina%20Depleled :type Float%20%28double-precision%29))
  (if (not (<= (Variables|Stamina|GetCurrent%20Stamina) 0.0))
    (Variables|Stamina|SetCurrent%20Stamina (- (Variables|Stamina|GetCurrent%20Stamina) Stamina%20Depleled))
    (CallFunction|UpdateStatsInfo)
    (if (<= (Variables|Stamina|GetCurrent%20Stamina) 0.0)
      _
      (else
        (return false))))
  (return true))

(fn IncreaseMaxStamina
  (params (Added%20Stamina :type Float%20%28double-precision%29))
  (Variables|Stamina|SetMax%20Stamina (+ (Variables|Stamina|GetMax%20Stamina) Added%20Stamina))
  (CallFunction|UpdateStatsInfo))

(fn IncreaseHealth
  (params (Added%20Health :type Float%20%28double-precision%29))
  (Variables|Health|SetCurrent%20Health (+ (Variables|Health|GetCurrent%20Health) Added%20Health))
  (if (> (Variables|Health|GetCurrent%20Health) (Variables|Health|GetMax%20Health))
    (Variables|Health|SetCurrent%20Health (Variables|Health|GetMax%20Health)))
  (CallFunction|UpdateStatsInfo))

(fn IncreaseStamina
  (params (Added%20Stamina :type Float%20%28double-precision%29))
  (Variables|Stamina|SetCurrent%20Stamina (+ (Variables|Stamina|GetCurrent%20Stamina) Added%20Stamina))
  (if (> (Variables|Stamina|GetCurrent%20Stamina) (Variables|Stamina|GetMax%20Stamina))
    (Variables|Stamina|SetCurrent%20Stamina (Variables|Stamina|GetMax%20Stamina)))
  (CallFunction|UpdateStatsInfo))

(fn IncreaseXP
  (params (Added%20XP :type Float%20%28double-precision%29))
  (Variables|XP|SetXP (+ (Variables|XP|GetXP) Added%20XP))
  (if (>= (Variables|XP|GetXP) (Variables|XP|GetMax%20XP))
    (LevelandXP|IncreaseLevel 1))
  (CallFunction|UpdateStatsInfo))

(fn IncreaseLevel
  (params (Added%20Level :type Integer))
  (Variables|XP|SetLevel (+ (Variables|XP|GetLevel) Added%20Level))
  (Variables|XP|SetMax%20XP (+ (Variables|XP|GetMax%20XP) 1.5e+02))
  (Variables|XP|SetXP 0.0)
  (CallFunction|UpdateStatsInfo))

(fn UpdateStatsInfo
  (Utilities|IsValid (Variables|Default|GetPlayer%20Character%20BP)
    (:Is%20Valid
      (Progress|SetPercent (Variables|/Game/UI/WB_HUD.WB_HUD_C|GetStaminaBar (Variables|/Game/ThirdPerson/Blueprints/BP_ThirdPersonCharacter.BP_ThirdPersonCharacter_C|GetHUD%20Widget (Variables|Default|GetPlayer%20Character%20BP))) (/ (Variables|Stamina|GetCurrent%20Stamina) (Variables|Stamina|GetMax%20Stamina)))
      (Progress|SetPercent (Variables|/Game/UI/WB_HUD.WB_HUD_C|GetHealthBar (Variables|/Game/ThirdPerson/Blueprints/BP_ThirdPersonCharacter.BP_ThirdPersonCharacter_C|GetHUD%20Widget (Variables|Default|GetPlayer%20Character%20BP))) (/ (Variables|Health|GetCurrent%20Health) (Variables|Health|GetMax%20Health)))
      (Progress|SetPercent (Variables|/Game/UI/WB_HUD.WB_HUD_C|GetXPBar (Variables|/Game/ThirdPerson/Blueprints/BP_ThirdPersonCharacter.BP_ThirdPersonCharacter_C|GetHUD%20Widget (Variables|Default|GetPlayer%20Character%20BP))) (/ (Variables|XP|GetXP) (Variables|XP|GetMax%20XP)))
      (Rendering|Components|TextRender|SetText (Variables|/Game/UI/WB_HUD.WB_HUD_C|GetXPText (Variables|/Game/ThirdPerson/Blueprints/BP_ThirdPersonCharacter.BP_ThirdPersonCharacter_C|GetHUD%20Widget (Variables|Default|GetPlayer%20Character%20BP))) (Utilities|Text|FormatText "{Current XP} / {Max XP}" (Variables|XP|GetXP) (Variables|XP|GetMax%20XP)))
      (Rendering|Components|TextRender|SetText (Variables|/Game/UI/WB_HUD.WB_HUD_C|GetLevelText (Variables|/Game/ThirdPerson/Blueprints/BP_ThirdPersonCharacter.BP_ThirdPersonCharacter_C|GetHUD%20Widget (Variables|Default|GetPlayer%20Character%20BP))) (Utilities|Text|ToText(Integer) (Variables|XP|GetLevel))))))