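; Boss AI controller that runs the boss behavior tree on BeginPlay and manages the boss health bar on screen.
; ActivateBossCombat creates the health bar widget and adds it to the viewport, while DeactivateBossCombat removes it and clears the reference.
; While the widget is valid, Tick polls Health over MaxHealth to set the bar's fill percent.
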(event Custom|Activate%20Boss%20Combat
  (bind _returnvalue (UserInterface|CreateWidget "/Game/UI/WB_Boss_HealthBar.WB_Boss_HealthBar_C"))
  (bind _output_get (Variables|Default|SetBoss%20Health%20Bar%20Widget _returnvalue))
  (UserInterface|Viewport|AddtoViewport _output_get 0))

(event Custom|Deactivate%20Boss%20Combat
  (Widget|RemovefromParent (Variables|Default|GetBoss%20Health%20Bar%20Widget))
  (Variables|Default|SetBoss%20Health%20Bar%20Widget 0))

(event EventBeginPlay
  (AI|RunBehaviorTree "/Game/AI/Boss/BT_AI_Boss.BT_AI_Boss"))

(event EventTick
  (params (DeltaSeconds :type Float%20%28single-precision%29))
  (bind _boss_health_bar_widget (Variables|Default|GetBoss%20Health%20Bar%20Widget)
    (:then
      (Progress|SetPercent (Variables|/Game/UI/WB_Boss_HealthBar.WB_Boss_HealthBar_C|GetHealthBar _boss_health_bar_widget) (/ (Variables|Default|Gethealth) (Variables|Default|GetmaxHealth))))
    (:else)))

(fn ConstructionScript
  (|CallParentFunction))